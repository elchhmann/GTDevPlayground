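; BP_AIBIG is a damageable AI target that takes BP_Bullet hits, bleeds, shows its health as text and ragdolls on death.
; AnyDamage subtracts bullet damage, accumulates bleeding, then drains health through a looping one-second Delay that never checks IsBleeding.
; Death turns the text red and enables mesh physics with velocities reset.
; Unless it bled out, a spine impulse along the player's forward vector follows.
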(event `self.ReceiveAnyDamage`
  (params (Damage :type "Float (single-precision)") (DamageType :type "DamageType Object Reference") (InstigatedBy :type "Controller Object Reference") (DamageCauser :type "Actor Object Reference"))
  (bind _health (`self.Health`))
  (bind _damage (`/Game/GTDP/Core/BP_Bullet.Damage` (`self.Bullet`)))
  (bind _startbleeding (`/Game/GTDP/Core/BP_Bullet.startBleeding` (`self.Bullet`)))
  (bind _asbp_bullet (cast `/Game/GTDP/Core/BP_Bullet` DamageCauser))
  (set `self.Bullet` _asbp_bullet)
  (set `self.BleedingAmount` (+ (`self.BleedingAmount`) (`/Game/GTDP/Core/BP_Bullet.BleedingMValue` (`self.Bullet`))))
  (set `self.Damage` _damage)
  (if _startbleeding
    (set `self.isBleeding` true))
  (bind _output_get (set `self.Health` (- (`self.Health`) (`self.Damage`))))
  (`TextRenderComponent.K2_SetText` (`self.HealthDisplay`) (`KismetTextLibrary.Conv_DoubleToText` (`self.Health`) "HalfToEven"))
  (set `self.BleedingAmount` (+ (`self.BleedingAmount`) (* 1.0 (`/Game/GTDP/Core/BP_Bullet.BleedingMValue` (`self.Bullet`)))))
  (`KismetSystemLibrary.PrintString` (`KismetStringLibrary.Conv_NameToString` (`/Game/GTDP/Core/BP_Bullet.HitArea` (`self.Bullet`))))
  (`KismetSystemLibrary.PrintString` "Hit Area:")
  (`KismetSystemLibrary.PrintString` (`KismetStringLibrary.Conv_DoubleToString` _damage))
  (`KismetSystemLibrary.PrintString` "Damage dealt:")
  (`KismetSystemLibrary.PrintString` (`KismetStringLibrary.Conv_BoolToString` _startbleeding))
  (`KismetSystemLibrary.PrintString` "Is Bleeding:")
  (`KismetSystemLibrary.PrintString` (`KismetStringLibrary.Conv_DoubleToString` (`self.BleedingAmount`)))
  (`KismetSystemLibrary.PrintString` "Bleeding Amount:")
  (`KismetSystemLibrary.PrintString` (`KismetStringLibrary.Conv_DoubleToString` _output_get))
  (`KismetSystemLibrary.PrintString` "Health")
  (if (not (< (`self.Health`) 0.0)) :!label _label
    (`KismetSystemLibrary.Delay` 1.0)
    (if (>= (`self.BleedingAmount`) (`self.Health`))
      (set `self.BledOut` true)
      (set `self.Health` 0.0)
      (else
        (set `self.Health` (- (`self.Health`) (`self.BleedingAmount`)))
        (`KismetSystemLibrary.PrintString` (`KismetStringLibrary.Conv_DoubleToString` _health))
        (`TextRenderComponent.K2_SetText` (`self.HealthDisplay`) (`KismetTextLibrary.Conv_DoubleToText` _health "HalfToEven"))
        (goto _label))))
  (`TextRenderComponent.SetTextRenderColor` (`self.HealthDisplay`) (make `Color` 0 0 255))
  (bind _asbp_character (cast `/Game/GTDP/Core/BP_Character` (`GameplayStatics.GetPlayerPawn` 0)))
  (set `self.Character` _asbp_character)
  (`KismetSystemLibrary.DelayUntilNextTick`)
  (`PrimitiveComponent.SetSimulatePhysics` (`self.SkeletalMesh`) true)
  (`PrimitiveComponent.SetAllPhysicsLinearVelocity` (`self.SkeletalMesh`) (0.0 0.0 0.0) false)
  (`PrimitiveComponent.SetAllPhysicsAngularVelocityInRadians` (`self.SkeletalMesh`) (0.0 0.0 0.0) false)
  (if (not (`self.BledOut`))
    (`PrimitiveComponent.AddImpulse` (`self.SkeletalMesh`) (* (`self.GetActorForwardVector` (`self.Character`)) (100.0 100.0 100.0)) "spine_05" false)
    (`PrimitiveComponent.SetCollisionResponseToChannel` (`self.SkeletalMesh`) "ECC_PhysicsBody" "ECR_Ignore")))

(event `self.ReceiveBeginPlay`
  (`TextRenderComponent.K2_SetText` (`self.HealthDisplay`) (`KismetTextLibrary.Conv_DoubleToText` (`self.Health`) "HalfToEven")))

(fn `UserConstructionScript`)