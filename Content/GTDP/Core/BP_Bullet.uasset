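; BP_Bullet is a bullet actor that deals damage and physical force to whatever its Sphere component hits.
; Each hit spawns an FS_MasterField at the bullet and triggers it with a radial magnitude, then applies Damage to the hit actor.
; Damage shrinks after every hit, so later impacts are weaker, and physics-simulating components receive an impulse from the bullet's velocity at its location.
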(event `self.ReceiveBeginPlay`)

(event `self.Sphere.OnComponentHit`
  (params (HitComponent :type "PrimitiveComponent Object Reference") (OtherActor :type "Actor Object Reference") (OtherComp :type "PrimitiveComponent Object Reference") (NormalImpulse :type "Vector Structure") (Hit :type "HitResult Structure (by ref)"))
  (set `self.Hit Actor` OtherActor)
  (bind _returnvalue (`|SpawnActorFromClass` "/Engine/EditorResources/FieldNodes/FS_MasterField.FS_MasterField_C" (`self.GetTransform`) "AlwaysSpawn" "MultiplyWithRoot" null null))
  (set `self.Field` _returnvalue)
  (set `/Engine/EditorResources/FieldNodes/FS_MasterField.ActivationType` "NewEnumerator4" (`self.Field`))
  (set `/Engine/EditorResources/FieldNodes/FS_MasterField.Radial Magnitude` 150.0 (`self.Field`))
  (`/Engine/EditorResources/FieldNodes/FS_MasterField.CE_Trigger` (`self.Field`))
  (`GameplayStatics.ApplyDamage` (`self.Hit Actor`) (`self.Damage`))
  (set `self.Damage` (* (`self.Damage`) 0.4))
  (if (`SceneComponent.IsSimulatingPhysics` OtherComp "None")
    (`PrimitiveComponent.AddImpulseAtLocation` OtherComp (`self.GetVelocity`) (`self.K2_GetActorLocation`) "None")))

(fn `UserConstructionScript`)