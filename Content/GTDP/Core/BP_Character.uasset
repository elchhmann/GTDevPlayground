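; First-person player character that handles movement, crouch, sprint, aim state and shooting with two weapons, a Honeybadger and a Glock17.
; Enhanced Input drives a delay-looped fire chain that spawns bullets and applies timeline camera recoil, reduced when crouched.
; Per-weapon ammo feeds timed reloads and slot switching, which calls SpawnInventory again to spawn and attach weapons to the arms.
; A short camera trace on Tick flags weapon lowering and blocks firing near obstacles.
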(event `EnhancedInput|/Game/GTDP/Data/IA_Reload`
  (params (ActionValue :type Boolean) (ElapsedSeconds :type "Float (double-precision)") (TriggeredSeconds :type "Float (double-precision)") (InputAction :type "InputAction Object Reference" :default "/Game/GTDP/Data/IA_Reload.IA_Reload"))
  (:`Triggered`
    (`/Engine/EditorBlueprintResources/StandardMacros.DoOnce` false :!label _label
      (:`Completed`
        (set `self.ReloadCheck` false)
        (`|ExecutionSequence`
          (:`then_0`
            (switch `int` (`self.EquippedWeaponIndex`)
              (:`0`
                (set `self.CheckedCurrentAmmo` (`self.HoneybadgerCurrentAmmunition`))
                (set `self.CheckedTotalAmmo` (`self.HoneybadgerTotalAmmunition`))
                (set `self.CheckedMagSize` (`self.HoneybadgerMagSize`)))
              (:`1`
                (set `self.CheckedCurrentAmmo` (`self.Glock17CurrentAmmunition`))
                (set `self.CheckedTotalAmmo` (`self.Glock17TotalAmmunition`))
                (set `self.CheckedMagSize` (`self.Glock17Magsize`)))))
          (:`then_1`
            (if (< (`self.CheckedCurrentAmmo`) (`self.CheckedMagSize`))
              (set `self.ReloadCheck` true)
              (if (>= (`self.CheckedTotalAmmo`) (- (`self.CheckedMagSize`) (`self.CheckedCurrentAmmo`)))
                (set `self.CheckedTotalAmmo` (- (`self.CheckedTotalAmmo`) (- (`self.CheckedMagSize`) (`self.CheckedCurrentAmmo`))))
                (set `self.CheckedCurrentAmmo` (`self.CheckedMagSize`))
                (else
                  (set `self.CheckedCurrentAmmo` (+ (`self.CheckedCurrentAmmo`) (`self.CheckedTotalAmmo`)))
                  (set `self.CheckedTotalAmmo` 0)))
              (`/Engine/EditorBlueprintResources/StandardMacros.Gate` false
                (:`Exit`
                  (set `self.isReloading` true)
                  (set `self.bCanFire` false)
                  (`KismetSystemLibrary.Delay` 2.0)
                  (set `self.isReloading` false)
                  (set `self.bCanFire` true)))
              (else
                (set `self.ReloadCheck` false))))
          (:`then_2`
            (if (`self.ReloadCheck`)
              (`KismetSystemLibrary.Delay` 2.0)
              (switch `int` (`self.EquippedWeaponIndex`)
                (:`0`
                  (set `self.CurrentAmmunition` (`self.CheckedCurrentAmmo`))
                  (set `self.HoneybadgerCurrentAmmunition` (`self.CheckedCurrentAmmo`))
                  (set `self.TotalAmmunition` (`self.CheckedTotalAmmo`))
                  (set `self.HoneybadgerTotalAmmunition` (`self.CheckedTotalAmmo`)))
                (:`1`
                  (set `self.CurrentAmmunition` (`self.CheckedCurrentAmmo`))
                  (set `self.Glock17CurrentAmmunition` (`self.CheckedCurrentAmmo`))
                  (set `self.TotalAmmunition` (`self.CheckedTotalAmmo`))
                  (set `self.Glock17TotalAmmunition` (`self.CheckedTotalAmmo`))))))))))
  (:`Completed`
    (goto _label :!via `Reset`)))

(event `EnhancedInput|/Game/GTDP/Data/IA_Fire`
  (params (ActionValue :type Boolean) (ElapsedSeconds :type "Float (double-precision)") (TriggeredSeconds :type "Float (double-precision)") (InputAction :type "InputAction Object Reference" :default "/Game/GTDP/Data/IA_Fire.IA_Fire"))
  (bind _output (`|GetArrayItem` (`self.EquippedWeapons`) (`self.EquippedWeaponIndex`)))
  (:`Triggered`
    (`/Engine/EditorBlueprintResources/StandardMacros.DoOnce` false :!label _label_2
      (:`Completed`
        (set `self.bHoldingFire` true)
        (if (`self.bHoldingFire`) :!label _label_3
          (if (`self.bCanFire`)
            (if (> (`self.CurrentAmmunition`) 0)
              (`AddComponent|NODE_AddAudioComponent-1`)
              (message `/Game/GTDP/Core/BPI_Glock17.Shoot` (`|GetArrayItem` (`self.EquippedWeapons`) (`self.EquippedWeaponIndex`)))
              (switch `int` (`self.EquippedWeaponIndex`)
                (:`0`
                  (`|PlayMontage` (`self.CharacterArms`) "/Game/GTDP/Art/Honeybadger/Animations/AM_firing.AM_firing"
                    (:`then`
                      _)))
                (:`1`
                  (`|PlayMontage` (`self.CharacterArms`) "/Game/GTDP/Art/Glock17/Animations/AM_Glock17_Fire.AM_Glock17_Fire"
                    (:`then`
                      _))))
              (`/Engine/EditorBlueprintResources/StandardMacros.Gate` false
                (:`Exit`
                  (bind _returnvalue (`|SpawnActorFromClass` "/Game/GTDP/Core/BP_Bullet.BP_Bullet_C" (`SceneComponent.K2_GetComponentToWorld` (`self.Camera`)) "AlwaysSpawn" "MultiplyWithRoot" null null))
                  (`PrimitiveComponent.IgnoreActorWhenMoving` (`self.CapsuleComponent`) _returnvalue true)
                  (`PrimitiveComponent.IgnoreActorWhenMoving` (`/Game/GTDP/Core/BP_Bullet.Sphere` _returnvalue) self true)
                  (`GameplayStatics.SpawnEmitterAtLocation` null (+ (`self.K2_GetActorLocation` _output) (* (`self.GetActorRightVector` _output) (300.0 300.0 300.0))))
                  (set `self.CurrentAmmunition` (- (`self.CurrentAmmunition`) 1))
                  (switch `int` (`self.EquippedWeaponIndex`)
                    (:`0`
                      (set `self.HoneybadgerCurrentAmmunition` (`self.CurrentAmmunition`)))
                    (:`1`
                      (set `self.Glock17CurrentAmmunition` (`self.CurrentAmmunition`))))
                  (`/Engine/EditorBlueprintResources/StandardMacros.Gate` false
                    (:`Exit`
                      (if (`self.isCrouching`)
                        (bind (_direction _vertical_recoil _horizontal_recoil) (`Timeline|Timeline` :!via `PlayFromStart`)
                          (:`Update`
                            (`self.Camera Recoil` (* _vertical_recoil 0.6) (* _horizontal_recoil 0.6))))
                        (else
                          (bind (_direction_2 _vertical_recoil_2 _horizontal_recoil_2) (`Timeline|Recoil Timeline` :!via `PlayFromStart`)
                            (:`Update`
                              (`self.Camera Recoil` _vertical_recoil_2 _horizontal_recoil_2)))))
                      (`/Engine/EditorBlueprintResources/StandardMacros.Gate` false
                        (:`Exit`
                          (`KismetSystemLibrary.Delay` (`self.HoneybadgerFireInterval`))
                          (if (not (`self.bSingleFire`))
                            (goto _label_3))))))))))))))
  (:`Completed`
    (set `self.bHoldingFire` false)
    (`KismetSystemLibrary.Delay` (`self.HoneybadgerFireInterval`))
    (goto _label_2 :!via `Reset`)))

(event `EnhancedInput|/Game/GTDP/Data/IA_SelectFire`
  (params (ActionValue :type Boolean) (ElapsedSeconds :type "Float (double-precision)") (TriggeredSeconds :type "Float (double-precision)") (InputAction :type "InputAction Object Reference" :default "/Game/GTDP/Data/IA_SelectFire.IA_SelectFire"))
  (:`Triggered`
    (`/Engine/EditorBlueprintResources/StandardMacros.DoOnce` false :!label _label_4
      (:`Completed`
        (switch `int` (`self.EquippedWeaponIndex`)
          (:`0`
            (`/Engine/EditorBlueprintResources/StandardMacros.FlipFlop`
              (:`A`
                (set `self.bSingleFire` true)
                (set `self.bSavedHoneybadgerSinglefire` true))
              (:`B`
                (set `self.bSingleFire` false)
                (set `self.bSavedHoneybadgerSinglefire` false))))
          (:`1`
            (set `self.bSingleFire` true))))))
  (:`Completed`
    (goto _label_4 :!via `Reset`)))

(event `EnhancedInput|/Game/GTDP/Data/IA_Movement`
  (params (ActionValue :type "Vector2D Structure") (ElapsedSeconds :type "Float (double-precision)") (TriggeredSeconds :type "Float (double-precision)") (InputAction :type "InputAction Object Reference" :default "/Game/GTDP/Data/IA_Movement.IA_Movement"))
  (bind (_x _y) (`KismetMathLibrary.BreakVector2D` (`self.Keyboard Input`)))
  (:`Triggered`
    (`|ExecutionSequence`
      (:`then_0`
        (set `self.Keyboard Input` ActionValue :!label _label_5)
        (`self.AddMovementInput` (* _y (`self.GetActorForwardVector`)))
        (`self.AddMovementInput` (* _x (`self.GetActorRightVector`))))
      (:`then_1`
        (set `self.isMoving` true))))
  (:`Completed`
    (`|ExecutionSequence`
      (:`then_0`
        (goto _label_5))
      (:`then_1`
        (set `self.isMoving` false)))))

(event `self.ReceiveBeginPlay`
  (`self.SpawnInventory`)
  ; Player UI
  (bind _returnvalue (`|CreateWidget` "/Game/GTDP/Core/WBP_PlayerUI.WBP_PlayerUI_C" (`GameplayStatics.GetPlayerController` 0)))
  (`UserWidget.AddToViewport` _returnvalue 0))

(event `EnhancedInput|/Game/GTDP/Data/IA_Camera`
  (params (ActionValue :type "Vector2D Structure") (ElapsedSeconds :type "Float (double-precision)") (TriggeredSeconds :type "Float (double-precision)") (InputAction :type "InputAction Object Reference" :default "/Game/GTDP/Data/IA_Camera.IA_Camera"))
  (bind (_x _y) (`KismetMathLibrary.BreakVector2D` (`self.Mouse Input`)))
  (:`Triggered`
    (set `self.Mouse Input` ActionValue :!label _label_6)
    (`self.AddControllerPitchInput` (* _y -1.0))
    (`self.AddControllerYawInput` _x))
  (:`Completed`
    (goto _label_6)))

(event `Custom Crouch`
  (set `self.isCrouching` true)
  (set `CharacterMovementComponent.MaxWalkSpeed` 150.0 (`self.CharacterMovement`))
  (bind (_direction _halfheight) (`Timeline|Custom Crouch Timeline` :!label _label_7)
    (:`Update`
      (`CapsuleComponent.SetCapsuleHalfHeight` (`self.CapsuleComponent`) _halfheight true))))

(event `EnhancedInput|/Game/GTDP/Data/IA_Slot1`
  (params (ActionValue :type Boolean) (ElapsedSeconds :type "Float (double-precision)") (TriggeredSeconds :type "Float (double-precision)") (InputAction :type "InputAction Object Reference" :default "/Game/GTDP/Data/IA_Slot1.IA_Slot1"))
  (:`Triggered`
    (if (not (`self.isReloading`))
      (`|ExecutionSequence`
        (:`then_0`
          (`/Engine/EditorBlueprintResources/StandardMacros.DoOnce` false :!label _label_8
            (:`Completed`
              (set `self.EquippedWeaponIndex` 0)
              (`self.SpawnInventory`)
              (set `self.CurrentAmmunition` (`self.HoneybadgerCurrentAmmunition`))
              (set `self.TotalAmmunition` (`self.HoneybadgerTotalAmmunition`))
              (`self.SetActorHiddenInGame` (`|GetArrayItem` (`self.EquippedWeapons`) (- 1 (`self.EquippedWeaponIndex`))) true)
              (set `self.bSingleFire` (`self.bSavedHoneybadgerSinglefire`)))))
        (:`then_1`
          (goto _label_9 :!via `Reset`))))))

(event `Custom UnCrouch`
  (set `self.isCrouching` false)
  (set `CharacterMovementComponent.MaxWalkSpeed` 300.0 (`self.CharacterMovement`))
  (goto _label_7 :!via `Reverse`))

(event `EnhancedInput|/Game/GTDP/Data/IA_Slot2`
  (params (ActionValue :type Boolean) (ElapsedSeconds :type "Float (double-precision)") (TriggeredSeconds :type "Float (double-precision)") (InputAction :type "InputAction Object Reference" :default "/Game/GTDP/Data/IA_Slot2.IA_Slot2"))
  (:`Triggered`
    (if (not (`self.isReloading`))
      (`|ExecutionSequence`
        (:`then_0`
          (`/Engine/EditorBlueprintResources/StandardMacros.DoOnce` false :!label _label_9
            (:`Completed`
              (set `self.EquippedWeaponIndex` 1)
              (`self.SpawnInventory`)
              (set `self.CurrentAmmunition` (`self.Glock17CurrentAmmunition`))
              (set `self.TotalAmmunition` (`self.Glock17TotalAmmunition`))
              (`self.SetActorHiddenInGame` (`|GetArrayItem` (`self.EquippedWeapons`) (- 1 (`self.EquippedWeaponIndex`))) true)
              (set `self.bSingleFire` true))))
        (:`then_1`
          (goto _label_8 :!via `Reset`))))))

(event `EnhancedInput|/Game/GTDP/Data/IA_Run`
  (params (ActionValue :type Boolean) (ElapsedSeconds :type "Float (double-precision)") (TriggeredSeconds :type "Float (double-precision)") (InputAction :type "InputAction Object Reference" :default "/Game/GTDP/Data/IA_Run.IA_Run"))
  (bind _charactermovement (`self.CharacterMovement`))
  (:`Triggered`
    (if (`self.isCrouching`)
      _
      (elif (`NavMovementComponent.IsFalling` (`self.CharacterMovement`))
        _
        (elif (not (`self.bAiming`))
          (set `CharacterMovementComponent.MaxWalkSpeed` 800.0 _charactermovement)
          (set `self.isRunning` true)
          (set `self.bCanFire` false)))))
  (:`Completed`
    (set `CharacterMovementComponent.MaxWalkSpeed` 300.0 _charactermovement)
    (set `self.isRunning` false)
    (set `self.bCanFire` true)))

(event `EnhancedInput|/Game/GTDP/Data/IA_Jump`
  (params (ActionValue :type Boolean) (ElapsedSeconds :type "Float (double-precision)") (TriggeredSeconds :type "Float (double-precision)") (InputAction :type "InputAction Object Reference" :default "/Game/GTDP/Data/IA_Jump.IA_Jump"))
  (:`Triggered`
    (if (not (`self.isCrouching`))
      (`self.Jump`))))

(event `self.ReceiveTick`
  (params (DeltaSeconds :type "Float (single-precision)"))
  (bind _camera (`self.Camera`))
  (`SceneComponent.K2_SetRelativeRotation` (`self.Pivot`) (`KismetMathLibrary.MakeRotator` 0.0 (.pitch (`self.GetControlRotation`))) false false)
  (bind (_outhit _returnvalue) (`KismetSystemLibrary.LineTraceSingle` (`SceneComponent.K2_GetComponentLocation` (`self.Camera`)) (+ (`SceneComponent.K2_GetComponentLocation` _camera) (* (`SceneComponent.GetForwardVector` _camera) (100.0 100.0 100.0))) "TraceTypeQuery1"))
  (set `self.lowerWeapon` _returnvalue)
  (if _returnvalue
    (if (`self.isRunning`)
      _
      (elif (not (`self.isReloading`))
        (set `self.bCanFire` false)))
    (elif (`self.isRunning`)
      _
      (elif (not (`self.isReloading`))
        (set `self.bCanFire` true)))))

(event `EnhancedInput|/Game/GTDP/Data/IA_Crouch`
  (params (ActionValue :type Boolean) (ElapsedSeconds :type "Float (double-precision)") (TriggeredSeconds :type "Float (double-precision)") (InputAction :type "InputAction Object Reference" :default "/Game/GTDP/Data/IA_Crouch.IA_Crouch"))
  (:`Triggered`
    (if (not (`NavMovementComponent.IsFalling` (`self.CharacterMovement`)))
      (`self.Custom Crouch`)))
  (:`Completed`
    (`self.Custom UnCrouch`)))

(event `EnhancedInput|/Game/GTDP/Data/IA_Aim`
  (params (ActionValue :type Boolean) (ElapsedSeconds :type "Float (double-precision)") (TriggeredSeconds :type "Float (double-precision)") (InputAction :type "InputAction Object Reference" :default "/Game/GTDP/Data/IA_Aim.IA_Aim"))
  (:`Triggered`
    (set `self.bAiming` true)
    (set `CharacterMovementComponent.MaxWalkSpeed` 300.0 (`self.CharacterMovement`)))
  (:`Completed`
    (set `self.bAiming` false)))

(fn `Camera Recoil`
  (params (`Vertical Recoil` :type "Float (double-precision)") (`Horizontal Recoil` :type "Float (double-precision)"))
  (`self.AddControllerPitchInput` `Vertical Recoil`)
  (`self.AddControllerYawInput` `Horizontal Recoil`))

(fn `SpawnInventory`
  (`EnhancedInputSubsystemInterface.AddMappingContext` (pcsubsystem `EnhancedInputLocalPlayerSubsystem` (`GameplayStatics.GetPlayerController` 0)) "/Game/GTDP/Data/IMC_FPS.IMC_FPS" 0 (struct))
  (for _array_element (`self.Inventory`)
    (bind _returnvalue (`|SpawnActorFromClass` _array_element (`KismetMathLibrary.MakeTransform` (0.0 0.0 0.0)) "Undefined" "MultiplyWithRoot" null null))
    (`KismetArrayLibrary.Array_Add` (`self.EquippedWeapons`) _returnvalue)
    (`self.K2_AttachToComponent` _returnvalue (`self.CharacterArms`) "ik_hand_gun" "KeepRelative" "KeepRelative" "KeepRelative" true)
    (`self.SetActorHiddenInGame` _returnvalue true))
  (`self.SetActorHiddenInGame` (`|GetArrayItem` (`self.EquippedWeapons`) (`self.EquippedWeaponIndex`)) false))

(fn `UserConstructionScript`)